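; FGDefaultPawnBP is a pawn Blueprint that executes moves passed to it through a DoMove event.
; Each move plays its animation through AttackAnim on the skeletal mesh's ThirdPerson_AnimBP.
; It then swaps the pawn's AI behavior by handing the move's behavior tree to ChangeBehaviour on the NPC_AI_BP controller.
; A debug string prints when the pawn has no such controller.
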(event `self.DoMove`
  (params (NewMove :type "FGMove Object Reference"))
  (`|ExecutionSequence`
    (:`then_0`
      (bind _asthird_person_anim_bp (cast `/Game/Mannequin/Animations/ThirdPerson_AnimBP` (`SkeletalMeshComponent.GetAnimInstance` (`self.SkeletalMesh`))))
      (`/Game/Mannequin/Animations/ThirdPerson_AnimBP.AttackAnim` _asthird_person_anim_bp (`FGMove.Animation` NewMove)))
    (:`then_1`
      (bind _asnpc_ai_bp (cast `/Game/zChangingBehaviour/NPC_AI_BP` (`AIBlueprintHelperLibrary.GetAIController` null))
        (:`then`
          (bind _asbehavior_tree (cast `BehaviorTree` (`FGMove.BehaviorTree` NewMove)))
          (`/Game/zChangingBehaviour/NPC_AI_BP.ChangeBehaviour` _asnpc_ai_bp _asbehavior_tree))
        (:`CastFailed`
          (`KismetSystemLibrary.PrintString` "bOOOOO"))))))

(fn `UserConstructionScript`)