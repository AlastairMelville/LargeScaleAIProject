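; BHDefaultPawn_BP is a pawn that performs a given move by playing its attack animation and switching its AI behaviour.
; The DoMove event passes the move's animation to AttackAnim on the ThirdPerson_AnimBP anim instance.
; It then hands the move's behavior tree to the NPC_AI_BP controller through ChangeBehaviour, printing debug strings on cast success or failure.
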(event `self.DoMove`
  (params (NewMove :type "Behaviour Object Reference"))
  (`|ExecutionSequence`
    (:`then_0`
      (bind _asthird_person_anim_bp (cast `/Game/Mannequin/Animations/ThirdPerson_AnimBP` (`SkeletalMeshComponent.GetAnimInstance` (`self.Mesh`))))
      (`/Game/Mannequin/Animations/ThirdPerson_AnimBP.AttackAnim` _asthird_person_anim_bp (`Behaviour.Animation` NewMove)))
    (:`then_1`
      (bind _asnpc_ai_bp (cast `/Game/zChangingBehaviour/NPC_AI_BP` (`AIBlueprintHelperLibrary.GetAIController` null))
        (:`then`
          (bind _asbehavior_tree (cast `BehaviorTree` (`Behaviour.BehaviorTree` NewMove)))
          (`/Game/zChangingBehaviour/NPC_AI_BP.ChangeBehaviour` _asnpc_ai_bp _asbehavior_tree)
          (`KismetSystemLibrary.PrintString` "Hello"))
        (:`CastFailed`
          (`KismetSystemLibrary.PrintString` "bOOOOO"))))))

(fn `UserConstructionScript`)